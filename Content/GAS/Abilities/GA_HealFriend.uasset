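; Gameplay ability that heals another pawn by launching a projectile at a player-confirmed target.
; A single-line trace target actor, filtered to pawns other than the avatar, supplies the end point.
; It reuses BP_FireballProjectile, spawned only on authority, to carry a GE_HealFriend spec with a SetByCaller health magnitude.
; The ability commits only after a successful spawn, then ends; cancelling targeting ends it without committing.
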(event `self.K2_ActivateAbility`
  (bind _returnvalue (`self.GetAvatarActorFromActorInfo`))
  (bind (_asynctaskproxy _data) (`AbilityTask_WaitTargetData.WaitTargetData` "None" "UserConfirmed" "/Script/GameplayAbilities.GameplayAbilityTargetActor_SingleLineTrace" 999999.0 (struct :`Name` "NoCollision") true (`self.MakeTargetLocationInfoFromOwnerActor`) (struct) null (`AbilitySystemBlueprintLibrary.MakeFilterHandle` (make `GameplayTargetDataFilter` "/Script/Engine.Pawn" "TDFS_NoSelf") (`self.GetAvatarActorFromActorInfo`)) true)
    (:`ValidData`
      (bind _returnvalue_2 (`AbilitySystemBlueprintLibrary.AssignTagSetByCallerMagnitude` (`self.MakeOutgoingGameplayEffectSpec` "/Game/GAS/Effects/Damage_Heal/GE_HealFriend.GE_HealFriend_C") (struct :`TagName` "GameplayAbilities.Effect.Health") 25.0))
      (`GameplayTask_SpawnActor.SpawnActor` null (`Actor.K2_GetActorLocation` _returnvalue) (struct) "/Game/BP_FireballProjectile.BP_FireballProjectile_C" true 2000.0 (`AbilitySystemBlueprintLibrary.GetTargetDataEndPoint` _data) _returnvalue_2 (cast `Pawn` _returnvalue :!pure true)
        (:`Success`
          (`self.K2_CommitAbility`)
          (`self.K2_EndAbility`))))
    (:`Cancelled`
      (`self.K2_EndAbility`))))